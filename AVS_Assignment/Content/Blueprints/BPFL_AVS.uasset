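; BPFL_AVS is a Blueprint function library with helpers for toggling player control state on the first local player.
; SetMovementLocked switches the player character's movement mode to None to freeze it, or back to Walking to release it.
; SetCursorUsage swaps between Game and UI input with a visible cursor and Game Only input with the cursor hidden.
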(fn SetMovementLocked
  (params (IsLocked :type Boolean))
  (bind _returnvalue (Game|GetPlayerCharacter 0))
  (bind _charactermovement (Variables|/Script/Engine.Character|GetCharacterMovement _returnvalue))
  (if IsLocked
    (Pawn|Components|CharacterMovement|SetMovementMode _charactermovement "MOVE_None" 0)
    (else
      (Pawn|Components|CharacterMovement|SetMovementMode _charactermovement "MOVE_Walking" 0))))

(fn SetCursorUsage
  (params (CursorRequired :type Boolean))
  (bind _returnvalue (Game|GetPlayerController 0))
  (if CursorRequired
    (Input|SetInputModeGameandUI _returnvalue 0 "DoNotLock" false false)
    (Variables|/Script/Engine.PlayerController|SetbShowMouseCursor _returnvalue true)
    (else
      (Input|SetInputModeGameOnly _returnvalue false)
      (Variables|/Script/Engine.PlayerController|SetbShowMouseCursor _returnvalue false)))
  (return))