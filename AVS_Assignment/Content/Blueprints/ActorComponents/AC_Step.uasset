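; Actor component that performs the Step ability, moving the player to a target location by sinking them below ground and raising them there.
; On BeginPlay it locks movement, turns the owner toward the target, switches to a temporary camera and expands cosmetic spheres at both ends.
; A Tick state machine runs timed linear eases for descent, ascent after a hidden teleport, and camera catch-up.
; It then restores control, collapses the spheres, signals completion and destroys itself.
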(event Custom|SpawnStepLocationSphere
  ;[0.1354 0 0.1239] Create BP_StepSpheres that are cosmetic
  (bind _returnvalue (Game|SpawnActorfromClass "/Game/Blueprints/Actors/BP_StepSphere.BP_StepSphere_C" (Math|Transform|MakeTransform (Variables|Default|GetStepLocation) "0, 0, 0" "1.000000,1.000000,1.000000") "AlwaysSpawn" "MultiplyWithRoot" 0 0))
  (bind _output_get (Variables|Default|SetStepSphereNewPosition _returnvalue))
  (Default|Expand _output_get)
  (Utilities|Time|SetTimerbyEvent (delegate Custom|DescendPlayer) 0.3))

(event Custom|DescendPlayer
  ;[0.15 0.15 0.15 0.5] Start moving the player through tick
  (Variables|Default|SetStepState "NewEnumerator1"))

(event Custom|MovePlayerToStepLocation
  ;[0.1141 0.1055 0.15 0.5] Move Player to new location while below ground
  (CallFunction|SetStepLocationDescended)
  (Transformation|SetActorLocation (Components|GetOwner) (Variables|Default|GetStepLocationDescended) false true)
  (CallFunction|AdjustStepLocation)
  (Variables|Default|SetStepState "NewEnumerator2"))

(event Custom|ShrinkComplete_New
  ;[0.5052 0.0484 0 0.5] Cleanup
  (Actor|DestroyActor (Variables|Default|GetStepSphereNewPosition))
  (Default|CallStepComplete)
  (Components|DestroyComponent))

(event Custom|ShrinkComplete_Original
  ;[0.5052 0.0484 0 0.5] Cleanup
  (Actor|DestroyActor (Variables|Default|GetStepSphereOriginalPosition)))

(event EventBeginPlay
  (bind _steplocation (Variables|Default|GetStepLocation))
  (bind _lookatrotation (CallFunction|GetPlayerLookatRotation _steplocation))
  ;[0.15 0.15 0.15 0.5] Prepare variables and face Step direction
  (CallFunction|SetMovementLocked true)
  (Variables|Default|SetStartLocation (Transformation|GetActorLocation (Components|GetOwner)))
  (CallFunction|SetOriginalDescentLocation)
  (CallFunction|CreateStepCamera)
  (Transformation|SetActorRotation (Components|GetOwner) (Math|Rotator|MakeRotator (.roll _lookatrotation) 0.0 (.yaw _lookatrotation)))
  ;[0.1354 0 0.1239] Create BP_StepSpheres that are cosmetic
  (bind _returnvalue (Game|SpawnActorfromClass "/Game/Blueprints/Actors/BP_StepSphere.BP_StepSphere_C" (Math|Transform|MakeTransform (CallFunction|GetOwnerFeetPosition) "0, 0, 0" "1.000000,1.000000,1.000000") "AlwaysSpawn" "MultiplyWithRoot" 0 0))
  (bind _output_get (Variables|Default|SetStepSphereOriginalPosition _returnvalue))
  (Default|Expand _output_get)
  (Utilities|Time|SetTimerbyEvent (delegate Custom|SpawnStepLocationSphere) 0.3))

(event EventTick
  (params (DeltaSeconds :type Float%20%28single-precision%29))
  (bind _alpha (CallFunction|SmoothTransition DeltaSeconds))
  (switch Utilities|FlowControl|Switch|SwitchonE_StepStates (Variables|Default|GetStepState)
    (:NewEnumerator1
      ;[0.2232 0.6354 0 0.5] Lower player below ground at StartLocation
      (Transformation|SetActorLocation (Components|GetOwner) (Math|Interpolation|Ease "Linear" _alpha (Variables|Default|GetStartLocation) (Variables|Default|GetDescentLocation)) false false)
      ;[0 0.15 0.02368 0.5] Reset time variables and trigger next phase of the Step ability
      (if (CallFunction|HasTimeElapsed)
        (Variables|Default|SetElapsedTime 0.0)
        (Variables|Default|SetStepState "NewEnumerator0")
        (CallFunction|MovePlayertoStepLocation)))
    (:NewEnumerator2
      ;[0.15 0.1211 0 0.5] Move player up above ground at StepLocation
      (Transformation|SetActorLocation (Components|GetOwner) (Math|Interpolation|Ease "Linear" _alpha (Variables|Default|GetStepLocationDescended) (Variables|Default|GetStepLocation)) false false)
      (if (CallFunction|HasTimeElapsed)
        (Variables|Default|SetMovementDuration 0.7)
        (Variables|Default|SetElapsedTime 0.0)
        (Variables|Default|SetStepState "NewEnumerator3")
        (Default|Collapse (Variables|Default|GetStepSphereOriginalPosition))
        ;[0.5052 0.0484 0 0.5] Cleanup
        (EventDispatchers|AssignShrinkComplete (Variables|Default|GetStepSphereOriginalPosition) (delegate Custom|ShrinkComplete_Original))))
    (:NewEnumerator3
      ;[0.15 0 0.009912 0.5] Move camera into the new position
      (Transformation|SetActorTransform (Variables|Default|GetStepTempCamera) (Math|Interpolation|Ease "Linear" _alpha (Variables|Default|GetStepCameraTransform) (Transformation|GetWorldTransform (Variables|Default|GetPlayerCamera))))
      ;[0 0.15 0.1465 0.5] Revert player to original state
      (if (CallFunction|HasTimeElapsed)
        (Variables|Default|SetStepState "NewEnumerator0")
        (Game|Player|SetViewTargetwithBlend (Game|GetPlayerController 0) (Components|GetOwner) 0.0 "VTBlend_Linear" 0.0 false)
        (CallFunction|SetMovementLocked false)
        (CallFunction|SetCursorUsage false)
        (Default|Collapse (Variables|Default|GetStepSphereNewPosition))
        (EventDispatchers|AssignShrinkComplete (Variables|Default|GetStepSphereNewPosition) (delegate Custom|ShrinkComplete_New))))))

(fn GetOwnerFeetPosition
  (bind _returnvalue (Components|GetOwner))
  (bind (_origin _boxextent) (Collision|GetActorBounds _returnvalue true false))
  (return (Math|Vector|MakeVector (.x _origin) (.y _origin) (- (.z _origin) (.z _boxextent)))))

(fn SetOriginalDescentLocation
  (bind _returnvalue (Components|GetOwner))
  (bind _startlocation (Variables|Default|GetStartLocation))
  (bind (_origin _boxextent) (Collision|GetActorBounds _returnvalue true false))
  (Variables|Default|SetDescentLocation (Math|Vector|MakeVector (.x _startlocation) (.y _startlocation) (- (.z _origin) (* (.z _boxextent) 2.0))))
  (return))

(fn CreateStepCamera
  (bind _output_get (Variables|Default|SetStepCameraTransform (Transformation|GetWorldTransform (Variables|Default|GetPlayerCamera))))
  (bind _returnvalue (Game|SpawnActorfromClass "/Script/Engine.CameraActor" _output_get "AlwaysSpawn" "MultiplyWithRoot" 0 0))
  (bind _output_get_2 (Variables|Default|SetStepTempCamera _returnvalue))
  (Class|CameraComponent|SetConstraintAspectRatio (Variables|/Script/Engine.CameraActor|GetCameraComponent _output_get_2) false)
  (Game|Player|SetViewTargetwithBlend (Game|GetPlayerController 0) _output_get_2 0.0 "VTBlend_Linear" 0.0 false)
  (return))

(fn AdjustStepLocation
  (Variables|Default|SetStepLocation (Math|Vector|MakeVector (.x (Variables|Default|GetStepLocation)) (.y (Variables|Default|GetStepLocation)) (+ (.z (Variables|Default|GetStepLocation)) (* (.z (.BoxExtent (Collision|GetActorBounds (Components|GetOwner) true false))) 1.2))))
  (return))

(fn SmoothTransition
  (params (DeltaSeconds :type Float%20%28double-precision%29))
  (bind _output_get (Variables|Default|SetElapsedTime (+ (Variables|Default|GetElapsedTime) DeltaSeconds)))
  (return (/ _output_get (Variables|Default|GetMovementDuration))))

(fn HasTimeElapsed
  (if (>= (Variables|Default|GetElapsedTime) (Variables|Default|GetMovementDuration))
    (return true)
    (else
      (return false))))

(fn SetStepLocationDescended
  (bind _steplocation (Variables|Default|GetStepLocation))
  (Variables|Default|SetStepLocationDescended (Math|Vector|MakeVector (.x _steplocation) (.y _steplocation) (- (.z _steplocation) (.z (.BoxExtent (Collision|GetActorBounds (Components|GetOwner) true false))))))
  (return))