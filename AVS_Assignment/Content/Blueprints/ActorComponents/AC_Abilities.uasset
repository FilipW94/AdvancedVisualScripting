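; Player ability component for BP_ThirdPersonCharacter that casts Projectile, Hedgehog, Rain, Step and Singularity from Enhanced Input actions.
; Projectile and Singularity require BP_TargetManager's main target, while Rain and Step toggle a cursor mode confirmed by left click.
; AC_CDManager gates casts, and Tick feeds remaining times to WBP_Abilities, switching itself off when no cooldowns remain.
; LightningFromAbove, ColdFeet and Hunger are empty stubs.
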(event Input|EnhancedActionEvents|EnhancedInputActionIA_Ability1
  (params (ActionValue :type Boolean) (ElapsedSeconds :type Float%20%28double-precision%29) (TriggeredSeconds :type Float%20%28double-precision%29) (InputAction :type Input%20Action%20Object%20Reference :default "/Game/Inputs/IA_Ability1.IA_Ability1"))
  ;[0.15 0.15 0.15 0.5] Abilities and their corresponding keybind. Check to see if player has the ability, not really used in this project
  (if (CallFunction|DoesPlayerHaveAbility "NewEnumerator0")
    (CallFunction|UseAbility "NewEnumerator0")))

(event Input|EnhancedActionEvents|EnhancedInputActionIA_Ability2
  (params (ActionValue :type Boolean) (ElapsedSeconds :type Float%20%28double-precision%29) (TriggeredSeconds :type Float%20%28double-precision%29) (InputAction :type Input%20Action%20Object%20Reference :default "/Game/Inputs/IA_Ability2.IA_Ability2"))
  ;[0.15 0.15 0.15 0.5] Abilities and their corresponding keybind. Check to see if player has the ability, not really used in this project
  (if (CallFunction|DoesPlayerHaveAbility "NewEnumerator6")
    (CallFunction|UseAbility "NewEnumerator6")))

(event Input|EnhancedActionEvents|EnhancedInputActionIA_LeftClick
  (params (ActionValue :type Boolean) (ElapsedSeconds :type Float%20%28double-precision%29) (TriggeredSeconds :type Float%20%28double-precision%29) (InputAction :type Input%20Action%20Object%20Reference :default "/Game/Inputs/IA_LeftClick.IA_LeftClick"))
  ;[0.15 0.15 0.15 0.5] Handle spells that require a mouse click to target
  (if (Variables|Default|GetMouseSelectInProgress)
    (switch Utilities|FlowControl|Switch|SwitchonE_Ability (Variables|Default|GetMouseTargetAbility)
      (:NewEnumerator2
        (CallFunction|UseRain))
      (:NewEnumerator1
        (CallFunction|UseStep)))))

(event Input|EnhancedActionEvents|EnhancedInputActionIA_Ability5
  (params (ActionValue :type Boolean) (ElapsedSeconds :type Float%20%28double-precision%29) (TriggeredSeconds :type Float%20%28double-precision%29) (InputAction :type Input%20Action%20Object%20Reference :default "/Game/Inputs/IA_Ability5.IA_Ability5"))
  ;[0.15 0.15 0.15 0.5] Abilities and their corresponding keybind. Check to see if player has the ability, not really used in this project
  (if (CallFunction|DoesPlayerHaveAbility "NewEnumerator9")
    (CallFunction|UseAbility "NewEnumerator9")))

(event Input|EnhancedActionEvents|EnhancedInputActionIA_Ability3
  (params (ActionValue :type Boolean) (ElapsedSeconds :type Float%20%28double-precision%29) (TriggeredSeconds :type Float%20%28double-precision%29) (InputAction :type Input%20Action%20Object%20Reference :default "/Game/Inputs/IA_Ability3.IA_Ability3"))
  ;[0.15 0.15 0.15 0.5] Abilities and their corresponding keybind. Check to see if player has the ability, not really used in this project
  (if (CallFunction|DoesPlayerHaveAbility "NewEnumerator2")
    (CallFunction|UseAbility "NewEnumerator2")))

(event Input|EnhancedActionEvents|EnhancedInputActionIA_Ability4
  (params (ActionValue :type Boolean) (ElapsedSeconds :type Float%20%28double-precision%29) (TriggeredSeconds :type Float%20%28double-precision%29) (InputAction :type Input%20Action%20Object%20Reference :default "/Game/Inputs/IA_Ability4.IA_Ability4"))
  ;[0.15 0.15 0.15 0.5] Abilities and their corresponding keybind. Check to see if player has the ability, not really used in this project
  (if (CallFunction|DoesPlayerHaveAbility "NewEnumerator1")
    (CallFunction|UseAbility "NewEnumerator1")))

(event EventBeginPlay
  (bind _asbp_third_person_character (Utilities|Casting|CastToBP_ThirdPersonCharacter (Components|GetOwner)))
  (Variables|Default|SetThirdPersonRef _asbp_third_person_character)
  (bind _returnvalue (Actor|GetActorOfClass "/Game/Blueprints/Actors/BP_TargetManager.BP_TargetManager_C"))
  (bind _output_get (Variables|Default|SetTargetManagerRef _returnvalue))
  (Utilities|IsValid _output_get
    (:Is%20Valid
      (CallFunction|FindCooldownManager)
      (CallFunction|SetupAbilityWidget))))

(event EventTick
  (params (DeltaSeconds :type Float%20%28single-precision%29))
  (bind _cooldownmanagerref (Variables|Default|GetCooldownManagerRef))
  (bind _abilitycooldownmap (Variables|/Game/Blueprints/ActorComponents/AC_CDManager.AC_CDManager_C|GetAbilityCooldownMap _cooldownmanagerref))
  ;[0.15 0.15 0.15 0.5] Update cooldowns every 0.1 sec
  (bind _keys (Utilities|Map|Keys _abilitycooldownmap))
  (if (Utilities|Array|IsNotEmpty _keys)
    (bind _values (Utilities|Map|Values _abilitycooldownmap))
    (for (_array_element _array_index) _values
      (Default|UpdateAbilityCooldown (Variables|Default|GetAbilityWidgetRef) (Utilities|Array|Get(acopy) _keys _array_index) (Utilities|Time|GetTimerRemainingTimebyHandle _array_element)))
    (else
      (Components|Tick|SetComponentTickEnabled false))))

(fn UseAbility
  (params (AbilityToUse :type E_Ability%20Enum :default "NewEnumerator0"))
  (if (Default|IsAbilityonCooldown (Variables|Default|GetCooldownManagerRef) AbilityToUse)
    (Development|PrintString "Ability on cooldown")
    (else
      (switch Utilities|FlowControl|Switch|SwitchonE_Ability AbilityToUse
        (:NewEnumerator0
          (CallFunction|UseBaseProjectile))
        (:NewEnumerator2
          (CallFunction|ToggleMouseInput AbilityToUse :!label _label))
        (:NewEnumerator1
          (goto _label))
        (:NewEnumerator9
          (Plannedbutnotimplemented|UseSingularity))
        (:NewEnumerator6
          (CallFunction|UseHedgehog))))))

(fn UseBaseProjectile
  (bind _targetmanagerref (Variables|Default|GetTargetManagerRef))
  (bind _currentmaintarget (Variables|/Game/Blueprints/Actors/BP_TargetManager.BP_TargetManager_C|GetCurrentMainTarget _targetmanagerref))
  (Utilities|IsValid _currentmaintarget
    (:Is%20Valid
      (Game|SpawnActorfromClass "/Game/Blueprints/Abilities/BP_Projectile_Base.BP_Projectile_Base_C" (Math|Transform|MakeTransform (Transformation|GetWorldLocation (Variables|/Game/ThirdPerson/Blueprints/BP_ThirdPersonCharacter.BP_ThirdPersonCharacter_C|GetBaseAbilitySpawn (Variables|Default|GetThirdPersonRef))) "0, 0, 0" "1.000000,1.000000,1.000000") "AlwaysSpawn" "MultiplyWithRoot" (Components|GetOwner) _currentmaintarget 0)
      (CallFunction|EnableTick)
      (Default|StartAbilityCooldown (Variables|Default|GetCooldownManagerRef) "NewEnumerator0"))
    (:Is%20Not%20Valid
      (Development|PrintString "Valid target needed"))))

(fn UseLightningfromAbove)

(fn UseRain
  (bind (_mouselocationfound _mouselocation) (CallFunction|FindMouseLocationinWorld 5e+03))
  (if _mouselocationfound
    (Game|SpawnActorfromClass "/Game/Blueprints/Abilities/BP_Rain.BP_Rain_C" (Math|Transform|MakeTransform (Math|Vector|MakeVector (.x _mouselocation) (.y _mouselocation) (+ (.z _mouselocation) 6e+02)) "0, 0, 0" "1.000000,1.000000,1.000000") "AlwaysSpawn" "MultiplyWithRoot" 0 0)
    (CallFunction|ClearMouseInput)
    (CallFunction|EnableTick)
    (Default|StartAbilityCooldown (Variables|Default|GetCooldownManagerRef) "NewEnumerator2")))

(fn UseColdFeet)

(fn FindCooldownManager
  (bind _output_get (Variables|Default|SetCooldownManagerRef (Actor|GetComponentbyClass (Components|GetOwner) "/Game/Blueprints/ActorComponents/AC_CDManager.AC_CDManager_C")))
  (Utilities|IsValid _output_get
    (:Is%20Valid
      (Development|PrintString "AC_Abilities: Cooldowmanager found on parent actor"))
    (:Is%20Not%20Valid
      (Development|PrintString "cooldownmanager not found"))))

(fn UseHedgehog
  (Class|BPIAnimationTrigger|AnimationTrigger(Message) (Components|SkeletalMesh|GetAnimInstance (Variables|/Script/Engine.Character|GetMesh (Game|GetPlayerCharacter 0))) "NewEnumerator6")
  (bind _returnvalue (Game|SpawnActorfromClass "/Game/Blueprints/Abilities/BP_Hedgehog.BP_Hedgehog_C" (Transformation|GetWorldTransform (Variables|/Game/ThirdPerson/Blueprints/BP_ThirdPersonCharacter.BP_ThirdPersonCharacter_C|GetBaseAbilitySpawn (Variables|Default|GetThirdPersonRef))) "AdjustIfPossibleButDontSpawnIfColliding" "MultiplyWithRoot" 0 (Variables|Default|GetTargetManagerRef) 0))
  (Utilities|IsValid _returnvalue
    (:Is%20Valid
      (Development|PrintString "Hedgehog spawned correctly")
      (CallFunction|EnableTick)
      (Default|StartAbilityCooldown (Variables|Default|GetCooldownManagerRef) "NewEnumerator6"))
    (:Is%20Not%20Valid
      (Development|PrintString "Hedgehog nog spawned correctly"))))

(fn SetupAbilityWidget
  (bind _returnvalue (UserInterface|CreateWidget "/Game/Widgets/WBP_Abilities.WBP_Abilities_C" (Game|GetPlayerController 0) (Variables|Default|GetAbilitiesAndKeybind)))
  (bind _output_get (Variables|Default|SetAbilityWidgetRef _returnvalue))
  (UserInterface|Viewport|AddtoViewport _output_get 0))

(fn DoesPlayerHaveAbility
  (params (AbilityToCheck :type E_Ability%20Enum :default "NewEnumerator7"))
  (bind _values (Utilities|Map|Values (Variables|Default|GetAbilitiesAndKeybind)))
  (if (Utilities|Array|ContainsItem _values AbilityToCheck)
    (return true)
    (else
      (return false))))

(fn UseSingularity
  (bind _targetmanagerref (Variables|Default|GetTargetManagerRef))
  (bind _targetmanagerref_2 (Variables|Default|GetTargetManagerRef))
  (bind _currentmaintarget (Variables|/Game/Blueprints/Actors/BP_TargetManager.BP_TargetManager_C|GetCurrentMainTarget _targetmanagerref))
  (bind _currentmaintarget_2 (Variables|/Game/Blueprints/Actors/BP_TargetManager.BP_TargetManager_C|GetCurrentMainTarget _targetmanagerref_2))
  (bind _returnvalue (Transformation|GetActorLocation _currentmaintarget))
  (bind _returnvalue_2 (+ (.z _returnvalue) 4.5e+02))
  (bind _returnvalue_3 (Math|Vector|MakeVector (.x _returnvalue) (.y _returnvalue) _returnvalue_2))
  (Utilities|IsValid _targetmanagerref
    (:Is%20Valid
      (Utilities|IsValid _currentmaintarget
        (:Is%20Valid
          (bind _closesttargetsarray (Default|FindClosestTargets _targetmanagerref _returnvalue_3 1.5e+03 10))
          (Utilities|IsValid _currentmaintarget_2
            (:Is%20Valid
              (Game|SpawnActorfromClass "/Game/Blueprints/Abilities/BP_Singularity.BP_Singularity_C" (Math|Transform|MakeTransform _returnvalue_3 "0, 0, 0" "1.000000,1.000000,1.000000") "Undefined" "MultiplyWithRoot" 0 _currentmaintarget_2 _closesttargetsarray 0)
              (Default|StartAbilityCooldown (Variables|Default|GetCooldownManagerRef) "NewEnumerator9"))
            (:Is%20Not%20Valid
              (Development|PrintString "Need a valid main target"))))))
    (:Is%20Not%20Valid
      (Development|PrintString "Need a valid main target"))))

(fn ClearMouseInput
  (Variables|Default|SetMouseTargetAbility "NewEnumerator7")
  (CallFunction|SetCursorUsage false)
  (Variables|Default|SetMouseSelectInProgress false))

(fn EnableTick
  (if (not (Class|ActorComponent|IsComponentTickEnabled))
    (Components|Tick|SetComponentTickEnabled true)
    (Development|PrintString "Tick Enabled")
    (return)))

(fn UseStep
  (bind (_mouselocationfound _mouselocation) (CallFunction|FindMouseLocationinWorld 5e+03))
  (if _mouselocationfound
    (Game|AddComponentbyClass (Components|GetOwner) "/Game/Blueprints/ActorComponents/AC_Step.AC_Step_C" (Variables|/Game/ThirdPerson/Blueprints/BP_ThirdPersonCharacter.BP_ThirdPersonCharacter_C|GetFollowCamera (Variables|Default|GetThirdPersonRef)) _mouselocation)
    (Default|StartAbilityCooldown (Variables|Default|GetCooldownManagerRef) "NewEnumerator1")
    (CallFunction|ClearMouseInput)
    (CallFunction|EnableTick)
    (else
      (Development|PrintString "AC_Abilities: Valid location for step was not found")
      (CallFunction|ClearMouseInput))))

(fn UseHunger)

(fn ToggleMouseInput
  (params (Ability :type E_Ability%20Enum :default "NewEnumerator7"))
  (if (Utilities|Enum|Equal(Enum) Ability (Variables|Default|GetMouseTargetAbility))
    (Variables|Default|SetMouseTargetAbility "NewEnumerator7")
    (CallFunction|SetCursorUsage false)
    (Variables|Default|SetMouseSelectInProgress false)
    (else
      (Variables|Default|SetMouseTargetAbility Ability)
      (CallFunction|SetCursorUsage true)
      (Variables|Default|SetMouseSelectInProgress true)))
  (return))