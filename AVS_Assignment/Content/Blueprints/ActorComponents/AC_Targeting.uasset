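; AC_Targeting is an actor component that gives third- or first-person player characters a toggleable camera lock-on to targets.
; The targeting input either clears the lock or searches ahead of the camera through BP_TargetManager, stepping outward with a growing radius to approximate a cone.
; While locked, Tick interpolates control rotation so the view follows the found target.
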(event Input|EnhancedActionEvents|EnhancedInputActionIA_TargetForward
  (params (ActionValue :type Boolean) (ElapsedSeconds :type Float%20%28double-precision%29) (TriggeredSeconds :type Float%20%28double-precision%29) (InputAction :type Input%20Action%20Object%20Reference :default "/Game/Inputs/IA_TargetForward.IA_TargetForward"))
  (if (Variables|Default|GetbFocusingTarget)
    (Variables|Default|SetbFocusingTarget false)
    (Default|ClearMainTarget (Variables|Default|GetTargetManagerRef))
    (else
      (CallFunction|FindFrontalTarget))))

(event EventBeginPlay
  (bind _asbp_third_person_character (Utilities|Casting|CastToBP_ThirdPersonCharacter (Components|GetOwner))
    (:then
      (Variables|Default|SetCameraBoomRef (Variables|/Game/ThirdPerson/Blueprints/BP_ThirdPersonCharacter.BP_ThirdPersonCharacter_C|GetCameraBoom _asbp_third_person_character))
      (Variables|Default|SetCameraRef (Variables|/Game/ThirdPerson/Blueprints/BP_ThirdPersonCharacter.BP_ThirdPersonCharacter_C|GetFollowCamera _asbp_third_person_character)))
    (:CastFailed
      (bind _asbp_first_person_character (Utilities|Casting|CastToBP_FirstPersonCharacter (Components|GetOwner)))
      (Variables|Default|SetCameraRef (Variables|/Game/FirstPerson/Blueprints/BP_FirstPersonCharacter.BP_FirstPersonCharacter_C|GetFirstPersonCamera _asbp_first_person_character))))
  (bind _returnvalue (Actor|GetActorOfClass "/Game/Blueprints/Actors/BP_TargetManager.BP_TargetManager_C"))
  (Variables|Default|SetTargetManagerRef _returnvalue))

(event EventTick
  (params (DeltaSeconds :type Float%20%28single-precision%29))
  (bind _cameraref (Variables|Default|GetCameraRef))
  (if (Variables|Default|GetbFocusingTarget)
    (Pawn|SetControlRotation (Game|GetPlayerController 0) (Math|Interpolation|RInterpTo (Transformation|GetWorldRotation _cameraref) (Math|Rotator|FindLookatRotation (Transformation|GetWorldLocation _cameraref) (Transformation|GetActorLocation (Variables|Default|GetCurrentTarget))) DeltaSeconds 1e+02))))

(fn GetCameraStartingPoint
  (return (Transformation|GetWorldLocation (Variables|Default|GetCameraRef))))

(fn GetForwardPoint
  (params (ForwardDistance :type Float%20%28double-precision%29))
  (return (* (Math|Vector|GetForwardVector (Variables|Default|GetCameraRef)) ForwardDistance)))

(fn SetFocusTarget
  (if (not (Variables|Default|GetbFocusingTarget))
    (Variables|/Script/Engine.SpringArmComponent|SetbUsePawnControlRotation (Variables|Default|GetCameraBoomRef) true)))

(fn FindFrontalTarget
  (bind _index (Utilities|FlowControl|ForLoopwithBreak 0 (Variables|Default|GetMaxNumberOfChecks) :!label _label)
    (:LoopBody
      (bind _closesttargetableactor (Default|FindClosestTargettoLocation (Variables|Default|GetTargetManagerRef) (+ (CallFunction|GetCameraStartingPoint) (CallFunction|GetForwardPoint (Math|Conversions|ToFloat(Integer) (* _index (Variables|Default|GetDistanceCheckIncrements))))) (* _index (Variables|Default|GetBaseTargetRadius))))
      (Utilities|IsValid _closesttargetableactor
        (:Is%20Valid
          (Variables|Default|SetCurrentTarget _closesttargetableactor)
          (Variables|Default|SetbFocusingTarget true)
          (goto _label Break))))))