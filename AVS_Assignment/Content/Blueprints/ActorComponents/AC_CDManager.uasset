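; Actor component that manages per-ability cooldowns, keyed by an ability enum.
; Starting a cooldown looks up its duration in a map, with a fallback default, and stores the timer handle in AbilityCooldownMap, whose entries mark abilities as on cooldown.
; Timers target functions by a name built from the enum string plus "_CooldownOver", so each ability has its own handler that removes its map entry.
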(event EventBeginPlay)

(event EventTick
  (params (DeltaSeconds :type Float%20%28single-precision%29)))

(fn RegisterAbilityCooldown
  (params (MatchingAbility :type E_Ability%20Enum :default "NewEnumerator0") (TimerHandle :type Timer%20Handle%20Structure))
  (Utilities|Map|Add (Variables|Default|GetAbilityCooldownMap) MatchingAbility TimerHandle)
  (return))

(fn IsAbilityonCooldown
  (params (Ability :type E_Ability%20Enum :default "NewEnumerator0"))
  (return (.ReturnValue (Utilities|Map|Find (Variables|Default|GetAbilityCooldownMap) Ability))))

(fn AbilityCooldownOver
  (params (AbilityHandleToRemove :type E_Ability%20Enum :default "NewEnumerator0"))
  (bind _returnvalue (Utilities|Map|Remove (Variables|Default|GetAbilityCooldownMap) AbilityHandleToRemove))
  (return _returnvalue))

(fn StartAbilityCooldown
  (params (Ability :type E_Ability%20Enum :default "NewEnumerator7"))
  (if (not (CallFunction|IsAbilityonCooldown Ability))
    (bind _returnvalue (Utilities|Time|SetTimerbyFunctionName 0 (Utilities|String|Append (Utilities|String|EnumtoString Ability) "_CooldownOver") (CallFunction|GetAbilityCooldownDuration Ability)))
    (CallFunction|RegisterAbilityCooldown Ability _returnvalue)))

(fn ProjectileCooldownOver
  (CallFunction|AbilityCooldownOver "NewEnumerator0"))

(fn LightningfromAboveCooldownOver
  (CallFunction|AbilityCooldownOver "NewEnumerator1"))

(fn SurroundandStingCooldownOver
  (CallFunction|AbilityCooldownOver "NewEnumerator2"))

(fn ColdFeetCooldownOver
  (CallFunction|AbilityCooldownOver "NewEnumerator3"))

(fn LeapCooldownOver
  (CallFunction|AbilityCooldownOver "NewEnumerator4"))

(fn HedgehogBallCooldownOver
  (CallFunction|AbilityCooldownOver "NewEnumerator6"))

(fn GetAbilityCooldownDuration
  (params (Ability :type E_Ability%20Enum :default "NewEnumerator7"))
  (bind _abilitycooldowndurations (Variables|Default|GetAbilityCooldownDurations))
  (bind (_value _returnvalue) (Utilities|Map|Find _abilitycooldowndurations Ability))
  (if _returnvalue
    (return _value)
    (else
      (return 5.0))))