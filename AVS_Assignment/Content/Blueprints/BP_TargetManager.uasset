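; BP_TargetManager tracks targetable actors, picks a main target and marks it in the world and on screen.
; It registers only BPI_Targetable actors, using their target message as the identifier in a lazily created WBP_TargetManagerUI list.
; A radius search loops the array for the actor closest to a given point and makes it the main target.
; Setting that target updates the widget and places a mesh marker above it; clearing hides the marker.
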(event EventBeginPlay
  (Development|SetHiddeninGame (Variables|Default|GetSM_TargetMarker) true false))

(fn ConstructionScript)

(fn AddTargettoArray
  (params (NewTarget :type Actor%20Object%20Reference))
  (if (Utilities|DoesObjectImplementInterface NewTarget "/Game/Blueprints/BPI_Targetable.BPI_Targetable_C")
    (Utilities|Array|Add (Variables|Default|GetTargetableActors) NewTarget)
    (bind _targetidentifier (Class|BPITargetable|GetTarget(Message) NewTarget))
    (CallFunction|ValidateWidget)
    (Default|AddTargettoList (Variables|Default|GetTargetManagerUIREF) (Utilities|Text|ToText(String) (Utilities|GetDisplayName NewTarget)) _targetidentifier)
    (return)))

(fn ValidateWidget
  (Utilities|IsValid (Variables|Default|GetTargetManagerUIREF)
    (:Is%20Valid
      (return))
    (:Is%20Not%20Valid
      (bind _returnvalue (UserInterface|CreateWidget "/Game/Widgets/WBP_TargetManagerUI.WBP_TargetManagerUI_C" (Game|GetPlayerController 0)))
      (bind _output_get (Variables|Default|SetTargetManagerUIREF _returnvalue))
      (UserInterface|Viewport|AddtoViewport _output_get 0)
      (return))))

(fn RemoveTargetfromArray
  (params (TargetToRemove :type Actor%20Object%20Reference))
  (bind _targetidentifier (Class|BPITargetable|GetTarget(Message) TargetToRemove))
  (CallFunction|ValidateWidget)
  (Default|RemoveTargetfromList (Variables|Default|GetTargetManagerUIREF) _targetidentifier)
  (bind _returnvalue (Utilities|Array|RemoveItem (Variables|Default|GetTargetableActors) TargetToRemove))
  (Development|PrintString (Utilities|String|ToString(Boolean) _returnvalue))
  (return))

(fn FindClosestTargettoLocation
  (params (SourcePoint :type Vector) (SearchRadius :type Float%20%28double-precision%29))
  (for _array_element (Variables|Default|GetTargetableActors)
    (if (<= (Math|Vector|Distance(Vector) SourcePoint (Transformation|GetActorLocation _array_element)) SearchRadius)
      (if (<= (Math|Vector|Distance(Vector) SourcePoint (Transformation|GetActorLocation _array_element)) (LocalVariables|GetCurrentMinDistance))
        (LocalVariables|SetCurrentMinDistance (Math|Vector|Distance(Vector) SourcePoint (Transformation|GetActorLocation _array_element)))
        (LocalVariables|SetCurrentClosestTarget (Transformation|GetActorLocation _array_element))
        (LocalVariables|SetClosestActor _array_element))))
  (Utilities|IsValid (LocalVariables|GetClosestActor)
    (:Is%20Valid
      (CallFunction|SetNewMainTarget (LocalVariables|GetClosestActor))
      (return (LocalVariables|GetClosestActor)))
    (:Is%20Not%20Valid
      (return 0))))

(fn SetNewMainTarget
  (params (PreviousMainTarget :type Actor%20Object%20Reference))
  (bind _returnvalue (Transformation|GetActorLocation PreviousMainTarget))
  (bind _targetidentifier (Class|BPITargetable|GetTarget(Message) PreviousMainTarget))
  (Default|SetMainTarget (Variables|Default|GetTargetManagerUIREF) (Utilities|Text|ToText(String) (Utilities|GetDisplayName PreviousMainTarget)) _targetidentifier)
  (Transformation|SetWorldLocation (Variables|Default|GetSM_TargetMarker) (Math|Vector|MakeVector (.x _returnvalue) (.y _returnvalue) (+ (.z _returnvalue) 1e+02)) false true)
  (Development|SetHiddeninGame (Variables|Default|GetSM_TargetMarker) false false))

(fn ClearMainTarget
  (Default|ClearOldMainTarget (Variables|Default|GetTargetManagerUIREF))
  (Development|SetHiddeninGame (Variables|Default|GetSM_TargetMarker) true false))