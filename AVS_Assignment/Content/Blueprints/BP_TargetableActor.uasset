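; BP_TargetableActor is a targetable actor that registers with BP_TargetManager while the player is within range and can receive damage.
; On BeginPlay it shows a random numeric identifier on a text component and caches the manager reference.
; A self-rescheduling one-second timer checks player distance, draws a red or green debug sphere, and adds or removes itself from the manager's array.
; DealDamage forwards damage to its ACHealth component.
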(event EventBeginPlay
  (CallFunction|RandomizeIdentifier)
  (Rendering|Components|TextRender|SetText (Variables|Default|GetTEXT_TargetIdentifier) (Variables|Default|GetTargetIdentifier))
  (bind _returnvalue (Actor|GetActorOfClass "/Game/Blueprints/BP_TargetManager.BP_TargetManager_C"))
  (Variables|Default|SetTargetManagerRef _returnvalue)
  (CallFunction|CheckifinPlayerRange))

(event EventDealDamage
  (params (DamageDealt :type Float%20%28double-precision%29))
  (Class|BPIDamageable|DealDamage(Message) (Variables|Default|GetAC_Health) DamageDealt))

(fn ConstructionScript)

(fn RandomizeIdentifier
  (Variables|Default|SetTargetIdentifier (Utilities|Text|ToText(String) (Utilities|String|ToString(Integer) (Math|Random|RandomIntegerinRange 0 999))))
  (return))

(fn CheckifinPlayerRange
  (if (>= (Math|Vector|Distance(Vector) (Transformation|GetActorLocation) (Transformation|GetActorLocation (Game|GetPlayerCharacter 0))) (Variables|Default|GetPlayerRange))
    (Rendering|Debug|DrawDebugSphere (Transformation|GetActorLocation) 1e+02 12 "(R=1.000000,G=0.030547,B=0.000000,A=1.000000)" 5.0)
    (CallFunction|NotinPlayerRange)
    (else
      (Rendering|Debug|DrawDebugSphere (Transformation|GetActorLocation) 1e+02 12 "(R=0.140633,G=1.000000,B=0.000000,A=1.000000)" 5.0)
      (CallFunction|InPlayerRange))))

(fn NotinPlayerRange
  (if (Utilities|Array|ContainsItem (Variables|/Game/Blueprints/BP_TargetManager.BP_TargetManager_C|GetTargetableActors (Variables|Default|GetTargetManagerRef)) self)
    (Default|RemoveTargetfromArray (Variables|Default|GetTargetManagerRef) self))
  (Utilities|Time|SetTimerbyFunctionName 0 "CheckIfInPlayerRange" 1.0))

(fn InPlayerRange
  (if (Utilities|Array|ContainsItem (Variables|/Game/Blueprints/BP_TargetManager.BP_TargetManager_C|GetTargetableActors (Variables|Default|GetTargetManagerRef)) self)
    _
    (else
      (Default|AddTargettoArray (Variables|Default|GetTargetManagerRef) self)))
  (Utilities|Time|SetTimerbyFunctionName 0 "CheckIfInPlayerRange" 1.0))

(fn GetTarget
  (return (Variables|Default|GetTargetIdentifier)))