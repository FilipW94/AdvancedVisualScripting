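; Base projectile actor that flies toward a target actor's position and deals damage to it.
; On BeginPlay it sets a lifespan and launches ProjectileMovement once along the spawn-to-target direction, without homing.
; Overlapping a BPI_Damageable actor damages the stored TargetActor, not necessarily the overlapped one; any overlap or hit destroys the projectile.
; A Timeline-lerp homing event, MoveToTarget, falls back to the last known position but is never triggered here.
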(event OnComponentBeginOverlap(SM_Projectile)
  (params (OverlappedComponent :type Primitive%20Component%20Object%20Reference) (OtherActor :type Actor%20Object%20Reference) (OtherComp :type Primitive%20Component%20Object%20Reference) (OtherBodyIndex :type Integer) (bFromSweep :type Boolean) (SweepResult :type Hit%20Result%20Structure%20%28by%20ref%29))
  (if (Utilities|DoesObjectImplementInterface OtherActor "/Game/Blueprints/Interfaces/BPI_Damageable.BPI_Damageable_C")
    (Class|BPIDamageable|DealDamage(Message) (Variables|Default|GetTargetActor) (Variables|Default|GetDamageDealth))
    (Actor|DestroyActor)
    (else
      (Development|PrintString "Hello")
      (Actor|DestroyActor))))

(event OnComponentHit(SM_Projectile)
  (params (HitComponent :type Primitive%20Component%20Object%20Reference) (OtherActor :type Actor%20Object%20Reference) (OtherComp :type Primitive%20Component%20Object%20Reference) (NormalImpulse :type Vector :default "0, 0, 0") (Hit :type Hit%20Result%20Structure%20%28by%20ref%29))
  (Development|PrintString "Hello")
  (Actor|DestroyActor))

(event Custom|MoveToTarget
  (bind _targetactor (Variables|Default|GetTargetActor))
  (bind _targetactor_2 (Variables|Default|GetTargetActor))
  (Utilities|IsValid _targetactor
    (:Is%20Valid
      (Variables|Default|SetEnemyLastPosition (Transformation|GetActorLocation _targetactor))
      (bind _lerptrack (Timeline|Timeline Play)
        (:Update
          (Utilities|IsValid (Variables|Default|GetTargetActor)
            (:Is%20Valid
              (Transformation|SetWorldLocation (Variables|Default|GetSM_Projectile) (Math|Vector|Lerp(Vector) (Variables|Default|GetSpawnLocation) (Transformation|GetActorLocation (Variables|Default|GetTargetActor)) _lerptrack) false false))
            (:Is%20Not%20Valid
              (Transformation|SetWorldLocation (Variables|Default|GetSM_Projectile) (Math|Vector|Lerp(Vector) (Variables|Default|GetSpawnLocation) (Variables|Default|GetEnemyLastPosition) _lerptrack) false false))))
        (:Finished
          (Utilities|IsValid _targetactor_2
            (:Is%20Valid
              (Class|BPIDamageable|DealDamage(Message) _targetactor_2 (Variables|Default|GetDamageDealth))
              (Actor|DestroyActor))
            (:Is%20Not%20Valid
              (Actor|DestroyActor))))))))

(event EventBeginPlay
  (Actor|SetLifeSpan 1e+01)
  (Variables|Default|SetSpawnLocation (Transformation|GetActorLocation))
  (Variables|Default|SetMoveProjectile true)
  (Variables|Default|SetEnemyLastPosition (Transformation|GetActorLocation (Variables|Default|GetTargetActor)))
  (CallFunction|SetProjectilePath))

(fn ConstructionScript)

(fn SetProjectilePath
  (Game|Components|ProjectileMovement|SetVelocityinLocalSpace (Variables|Default|GetProjectileMovement) (* (Math|Vector|Normalize (- (Variables|Default|GetEnemyLastPosition) (Variables|Default|GetSpawnLocation))) 1.2e+03)))