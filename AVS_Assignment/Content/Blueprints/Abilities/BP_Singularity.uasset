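; BP_Singularity is an ability actor that grows a singularity mesh and Niagara effect, then captures targets in range.
; A timeline scales both up after a short delay while the actor turns toward the player.
; Each entry in TargetsInRange gets a spawned BP_SingularityPivot snapped to the mesh, with the target attached.
; If targets exist, a timer later hides the effect and reverses the timeline, destroying the actor when finished.
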(event Custom|IncraseSize
  (bind (_direction _sizetrack) (Timeline|SingularityTimeline PlayFromStart)
    (:Update
      (Transformation|SetWorldScale3D (Variables|Default|GetSM_Singularity) (Math|Vector|Lerp(Vector) (Variables|Default|GetMeshStartSize) (Variables|Default|GetMeshEndsize) _sizetrack))
      (Transformation|SetWorldScale3D (Variables|Default|GetNS_Singularity) (Math|Vector|Lerp(Vector) (Variables|Default|GetEmitterStartSize) (Variables|Default|GetEmitterEndSize) _sizetrack)))
    (:Finished
      (switch Utilities|FlowControl|Switch|SwitchonETimelineDirection _direction
        (:Forward
          (CallFunction|LocatedTargets))
        (:Backward
          (Actor|DestroyActor))))))

(event Custom|LocatedTargets
  (if (Utilities|Array|IsNotEmpty (Variables|Default|GetTargetsInRange))
    (for _array_element (Variables|Default|GetTargetsInRange)
      (CallFunction|CreatePivotforTarget _array_element))
    (Development|PrintString (Utilities|String|Append "Targets: " (Utilities|String|ToString(Integer) (Utilities|Array|Length (Variables|Default|GetTargetsInRange))) "Pivots: " (Utilities|String|ToString(Integer) (Utilities|Array|Length (Variables|Default|GetPivotArray)))))
    (Utilities|Time|SetTimerbyEvent (delegate Custom|ReduceSize) 5.0)))

(event Custom|ReduceSize
  (Development|SetHiddeninGame (Variables|Default|GetNS_Singularity) true false)
  (bind (_direction _sizetrack) (Timeline|SingularityTimeline ReverseFromEnd)
    (:Update
      (Transformation|SetWorldScale3D (Variables|Default|GetSM_Singularity) (Math|Vector|Lerp(Vector) (Variables|Default|GetMeshStartSize) (Variables|Default|GetMeshEndsize) _sizetrack))
      (Transformation|SetWorldScale3D (Variables|Default|GetNS_Singularity) (Math|Vector|Lerp(Vector) (Variables|Default|GetEmitterStartSize) (Variables|Default|GetEmitterEndSize) _sizetrack)))
    (:Finished
      (switch Utilities|FlowControl|Switch|SwitchonETimelineDirection _direction
        (:Forward
          (CallFunction|LocatedTargets))
        (:Backward
          (Actor|DestroyActor))))))

(event EventBeginPlay
  (Utilities|FlowControl|Delay 1.0)
  (CallFunction|IncraseSize)
  (Transformation|SetActorRotation (CallFunction|GetPlayerLookatRotation (Transformation|GetActorLocation))))

(fn ConstructionScript)

(fn CreatePivotforTarget
  (params (Target :type Actor%20Object%20Reference))
  (bind _returnvalue (Game|SpawnActorfromClass "/Game/Blueprints/Actors/BP_SingularityPivot.BP_SingularityPivot_C" (Math|Transform|MakeTransform (Transformation|GetWorldLocation (Variables|Default|GetSM_Singularity)) "0, 0, 0" "1.000000,1.000000,1.000000") "AlwaysSpawn" "MultiplyWithRoot" self (Transformation|GetActorLocation Target) Target 0))
  (Transformation|AttachComponentToComponent _returnvalue (Variables|Default|GetSM_Singularity) "None" "SnapToTarget" "KeepWorld" "KeepWorld" true)
  (Transformation|AttachComponentToComponent Target (Variables|/Game/Blueprints/Actors/BP_SingularityPivot.BP_SingularityPivot_C|GetSingularityPivot _returnvalue) "None" "KeepWorld" "KeepRelative" "KeepWorld" false)
  (Utilities|Array|Add (Variables|Default|GetPivotArray) (Variables|/Game/Blueprints/Actors/BP_SingularityPivot.BP_SingularityPivot_C|GetSingularityPivot _returnvalue)))