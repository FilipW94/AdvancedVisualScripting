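; BP_Hedgehog is an ability actor that launches homing-style quills at up to five nearby targets.
; It dissolves in while a timeline moves and rotates the mesh along a spline, then queries TargetManagerRef for closest targets and spawns one BP_HedgehogQuill per target.
; A Tick sphere trace halts movement and fades it out when blocked.
; The reversed disintegrate timeline destroys the actor after blocking, finding no targets, or a post-spawn delay.
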(event Custom|MoveHedgehogIntoPosition
  (bind _output_get (Variables|Default|SetStartRotation (Variables|/Script/Engine.SceneComponent|GetRelativeRotation (Variables|Default|GetSM_Hedgehog))))
  (Variables|Default|SetEndRotation (Math|Rotator|MakeRotator (+ (.roll _output_get) 1.8e+02) (.pitch _output_get) (.yaw _output_get)))
  (bind _newtrack_0 (Timeline|HedgehogTimeline PlayFromStart)
    (:Update
      (Transformation|SetRelativeLocationAndRotation (Variables|Default|GetSM_Hedgehog) (Spline|GetLocationatTime (Variables|Default|GetSpline) _newtrack_0 "Local" false) (Math|Rotator|Lerp(Rotator) (Variables|Default|GetStartRotation) (Variables|Default|GetEndRotation) _newtrack_0 true) false false))
    (:Finished
      (CallFunction|FindClosestHedgehogTargets))))

(event Custom|WaitForCompletion
  (Utilities|FlowControl|Delay 2.5)
  (CallFunction|MaterialFadeOut))

(event Custom|MaterialFadeIn
  (bind _sm_hedgehog (Variables|Default|GetSM_Hedgehog))
  (bind _returnvalue (Rendering|Material|CreateDynamicMaterialInstance _sm_hedgehog 0 (Rendering|Material|GetMaterial _sm_hedgehog 0) "None" :!class /Script/Engine.PrimitiveComponent))
  (Variables|Default|SetDisintMaterial _returnvalue)
  (bind (_direction _scalartrack) (Timeline|DisintegrateTimeline PlayFromStart)
    (:Update
      (Rendering|Material|SetScalarParameterValue (Variables|Default|GetDisintMaterial) "Amount" (Math|Float|Lerp 1.0 0.0 _scalartrack) :!class /Script/Engine.MaterialInstanceDynamic))
    (:Finished
      (switch Utilities|FlowControl|Switch|SwitchonETimelineDirection _direction
        (:Forward
          (Rendering|Material|SetOverlayMaterial (Variables|Default|GetSM_Hedgehog) "/Game/Materials/MI_Outline_Hedgehog.MI_Outline_Hedgehog" :!class /Script/Engine.MeshComponent))
        (:Backward
          (Actor|DestroyActor))))))

(event Custom|MaterialFadeOut
  (Rendering|Material|SetOverlayMaterial (Variables|Default|GetSM_Hedgehog) 0 :!class /Script/Engine.MeshComponent)
  (bind (_direction _scalartrack) (Timeline|DisintegrateTimeline ReverseFromEnd)
    (:Update
      (Rendering|Material|SetScalarParameterValue (Variables|Default|GetDisintMaterial) "Amount" (Math|Float|Lerp 1.0 0.0 _scalartrack) :!class /Script/Engine.MaterialInstanceDynamic))
    (:Finished
      (switch Utilities|FlowControl|Switch|SwitchonETimelineDirection _direction
        (:Forward
          (Rendering|Material|SetOverlayMaterial (Variables|Default|GetSM_Hedgehog) "/Game/Materials/MI_Outline_Hedgehog.MI_Outline_Hedgehog" :!class /Script/Engine.MeshComponent))
        (:Backward
          (Actor|DestroyActor))))))

(event EventBeginPlay
  (Utilities|FlowControl|Delay 0.2)
  (CallFunction|MaterialFadein)
  (CallFunction|MoveHedgehogIntoPosition))

(event EventTick
  (params (DeltaSeconds :type Float%20%28single-precision%29))
  (bind _sm_hedgehog (Variables|Default|GetSM_Hedgehog))
  (bind _returnvalue (Transformation|GetWorldLocation _sm_hedgehog))
  (if (not (Variables|Default|GetBlocked))
    (bind _returnvalue_2 (Collision|SphereTraceForObjects _returnvalue _returnvalue 55.0 (Variables|Default|GetObject%20Types) false 0 "None" true "(R=1.000000,G=0.000000,B=0.000000,A=1.000000)" "(R=0.000000,G=1.000000,B=0.000000,A=1.000000)" 1.0))
    (if _returnvalue_2
      (Utilities|FlowControl|Sequence
        (:then_0
          (Variables|Default|SetBlocked true)
          (bind _newtrack_0 (Timeline|HedgehogTimeline Stop)
            (:Update
              (Transformation|SetRelativeLocationAndRotation (Variables|Default|GetSM_Hedgehog) (Spline|GetLocationatTime (Variables|Default|GetSpline) _newtrack_0 "Local" false) (Math|Rotator|Lerp(Rotator) (Variables|Default|GetStartRotation) (Variables|Default|GetEndRotation) _newtrack_0 true) false false))
            (:Finished
              (CallFunction|FindClosestHedgehogTargets))))
        (:then_1
          (CallFunction|MaterialFadeOut))))))

(fn ConstructionScript)

(fn SpawnQuill
  (if (Utilities|Array|IsNotEmpty (Variables|Default|GetHedgehogTargets))
    (for _array_element (Variables|Default|GetHedgehogTargets)
      (bind _returnvalue (Game|SpawnActorfromClass "/Game/Blueprints/Abilities/BP_HedgehogQuill.BP_HedgehogQuill_C" (Math|Transform|MakeTransform (.location (Transformation|GetWorldTransform (Variables|Default|GetSM_Hedgehog))) "0, 0, 0" "1.000000,1.000000,1.000000") "AlwaysSpawn" "MultiplyWithRoot" 0 _array_element (Variables|Default|GetHedgehogTargets) 0))
      (Utilities|IsValid _returnvalue
        (:Is%20Valid
          (Development|PrintString "Quill spawned"))
        (:Is%20Not%20Valid
          (Development|PrintString "BP_Hedgehog: Quill did not spawn properly"))))
    (CallFunction|WaitforCompletion)))

(fn FindClosestHedgehogTargets
  (bind _targetmanagerref (Variables|Default|GetTargetManagerRef))
  (Utilities|IsValid _targetmanagerref
    (:Is%20Valid
      (bind _closesttargetsarray (Default|FindClosestTargets _targetmanagerref (Transformation|GetWorldLocation (Variables|Default|GetSM_Hedgehog)) 2e+03 5))
      (if (Utilities|Array|IsNotEmpty _closesttargetsarray)
        (Variables|Default|SetHedgehogTargets _closesttargetsarray)
        (CallFunction|SpawnQuill)
        (else
          (CallFunction|MaterialFadeOut))))
    (:Is%20Not%20Valid
      (CallFunction|MaterialFadeOut))))