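; BP_RainSpike is a falling spike projectile that damages what it hits on the way down.
; On BeginPlay a timeline lerps it straight down a fixed distance from its start height with a swept move.
; A mesh hit sets a flag that halts the timeline and sends a damage message to actors implementing BPI_Damageable.
; The spike destroys itself on a short timer after a hit or when the fall finishes.
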(event OnComponentHit(SM_Spike)
  (params (HitComponent :type Primitive%20Component%20Object%20Reference) (OtherActor :type Actor%20Object%20Reference) (OtherComp :type Primitive%20Component%20Object%20Reference) (NormalImpulse :type Vector :default "0, 0, 0") (Hit :type Hit%20Result%20Structure%20%28by%20ref%29))
  (Variables|Default|SetTargetHit true)
  (if (Utilities|DoesObjectImplementInterface OtherActor "/Game/Blueprints/Interfaces/BPI_Damageable.BPI_Damageable_C")
    (Class|BPIDamageable|DealDamage(Message) OtherActor 2.0)
    (Actor|Tick|SetActorTickEnabled false)
    (Utilities|Time|SetTimerbyFunctionName 0 "CleanupSpike" 2.0)))

(event Custom|StartSpikeTimeline
  (bind _startposition (Variables|Default|GetStartPosition))
  (bind _spiketrack (Timeline|SpikeTimeline Play)
    (:Update
      (if (Variables|Default|GetTargetHit)
        (CallFunction|StopSpikeTimeline)
        (Utilities|Time|SetTimerbyFunctionName 0 "CleanupSpike" 2.0)
        (else
          (Transformation|SetActorLocation (Math|Vector|MakeVector (.x _startposition) (.y _startposition) (Math|Float|Lerp (.z _startposition) (- (.z _startposition) 2e+03) _spiketrack)) true false))))
    (:Finished
      (Utilities|Time|SetTimerbyFunctionName 0 "CleanupSpike" 2.0))))

(event Custom|StopSpikeTimeline
  (bind _startposition (Variables|Default|GetStartPosition))
  (bind _spiketrack (Timeline|SpikeTimeline Stop)
    (:Update
      (if (Variables|Default|GetTargetHit)
        (CallFunction|StopSpikeTimeline)
        (Utilities|Time|SetTimerbyFunctionName 0 "CleanupSpike" 2.0)
        (else
          (Transformation|SetActorLocation (Math|Vector|MakeVector (.x _startposition) (.y _startposition) (Math|Float|Lerp (.z _startposition) (- (.z _startposition) 2e+03) _spiketrack)) true false))))
    (:Finished
      (Utilities|Time|SetTimerbyFunctionName 0 "CleanupSpike" 2.0))))

(event EventBeginPlay
  (Variables|Default|SetStartPosition (Transformation|GetWorldLocation (Variables|Default|GetSM_Spike)))
  (CallFunction|StartSpiketimeline))

(fn ConstructionScript)

(fn CleanupSpike
  (Actor|DestroyActor))