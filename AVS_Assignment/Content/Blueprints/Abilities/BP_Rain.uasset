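; BP_Rain is an ability actor that rains spikes from a cloud mesh.
; On BeginPlay it starts a self-rescheduling timer event that spawns a BP_RainSpike at a random horizontal offset around the cloud, slightly below it.
; A counter tracks spawned spikes, and the actor destroys itself once it reaches SpikeToSpawn.
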(event Custom|SpawnSpikes
  (bind _sm_cloud (Variables|Default|GetSM_Cloud))
  (bind _returnvalue (Transformation|GetWorldLocation _sm_cloud))
  (if (>= (Variables|Default|GetSpikeCount) (Variables|Default|GetSpikeToSpawn))
    (Actor|DestroyActor)
    (else
      (Game|SpawnActorfromClass "/Game/Blueprints/Abilities/BP_RainSpike.BP_RainSpike_C" (Math|Transform|MakeTransform (Math|Vector|MakeVector (+ (.x _returnvalue) (Math|Random|RandomFloatinRange -1.5e+02 1.5e+02)) (+ (.y _returnvalue) (Math|Random|RandomFloatinRange -1.5e+02 1.5e+02)) (- (.z _returnvalue) 4e+01)) "0, 0, 0" "1.000000,1.000000,1.000000") "AlwaysSpawn" "MultiplyWithRoot" 0 0)
      (bind _result (Math|Integer|IncrementInt (Variables|Default|GetSpikeCount))
        (:%20%20
          (Variables|Default|SetSpikeCount _result)
          (Utilities|Time|SetTimerbyEvent (delegate Custom|SpawnSpikes) 0.1))))))

(event EventBeginPlay
  (Variables|Default|SetSpikeCount 0)
  (CallFunction|SpawnSpikes))

(fn ConstructionScript)