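; BP_HedgehogQuill is a hedgehog ability projectile that stretches from its spawn point to one target, retracts and then deals damage.
; On BeginPlay it line traces to the target, ignoring the other quill targets, and destroys itself if the view is blocked.
; Otherwise it rotates toward the target, and a timeline scales the mesh's Z to the hit distance.
; After a brief hold the timeline reverses, applying damage and destroying the quill when retraction finishes.
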(event Custom|ReturnQuill
  (bind _sm_quill (Variables|Default|GetSM_Quill))
  (bind _returnvalue (Transformation|GetWorldScale _sm_quill))
  (bind (_direction _quillextentiontrack) (Timeline|AlterQuill ReverseFromEnd)
    (:Update
      (Utilities|IsValid (Variables|Default|GetSM_Quill)
        (:Is%20Valid
          (Transformation|SetWorldScale3D (Variables|Default|GetSM_Quill) (Math|Vector|MakeVector (.x _returnvalue) (.y _returnvalue) (Math|Float|Lerp 0.05 (Variables|Default|GetDistanceToTarget) _quillextentiontrack))))
        (:Is%20Not%20Valid
          (Actor|DestroyActor))))
    (:Finished
      (Utilities|IsValid (Variables|Default|GetSM_Quill)
        (:Is%20Valid
          (switch Utilities|FlowControl|Switch|SwitchonETimelineDirection _direction
            (:Forward
              (Utilities|FlowControl|Delay 1.0)
              (CallFunction|ReturnQuill))
            (:Backward
              (Class|BPIDamageable|DealDamage(Message) (Variables|Default|GetQuillTarget) (Variables|Default|GetQuillDamage))
              (Actor|DestroyActor))))
        (:Is%20Not%20Valid
          (Actor|DestroyActor))))))

(event Custom|AimAtTarget
  (Variables|Default|SetTargetLocation (Transformation|GetActorLocation (Variables|Default|GetQuillTarget)))
  (bind _outhit (Collision|LineTraceByChannel (Transformation|GetActorLocation) (Variables|Default|GetTargetLocation) "TraceTypeQuery3" false (Variables|Default|GetAllQuillTargets) "None"))
  (if (and (.bblockinghit _outhit) (== (.hitactor _outhit) (Variables|Default|GetQuillTarget)))
    (Variables|Default|SetDistanceToTarget (+ (* (.distance _outhit) 0.01) 1.0))
    ;[0.15 0.15 0.15 0.5] Face target
    (Transformation|SetRelativeRotation (Variables|Default|GetScene) (Math|Rotator|FindRelativeLookatRotation (Transformation|GetActorTransform) (Variables|Default|GetTargetLocation)) false false)
    (CallFunction|AlterQuillShape)
    (else
      ;[0.15 0.15 0.15 0.5] Quills are spawned even if the target is out of sight. Destroy if blocked
      (Actor|DestroyActor))))

(event Custom|AlterQuillShape
  (bind _sm_quill (Variables|Default|GetSM_Quill))
  (bind _returnvalue (Transformation|GetWorldScale _sm_quill))
  (bind (_direction _quillextentiontrack) (Timeline|AlterQuill PlayFromStart)
    (:Update
      (Utilities|IsValid (Variables|Default|GetSM_Quill)
        (:Is%20Valid
          (Transformation|SetWorldScale3D (Variables|Default|GetSM_Quill) (Math|Vector|MakeVector (.x _returnvalue) (.y _returnvalue) (Math|Float|Lerp 0.05 (Variables|Default|GetDistanceToTarget) _quillextentiontrack))))
        (:Is%20Not%20Valid
          (Actor|DestroyActor))))
    (:Finished
      (Utilities|IsValid (Variables|Default|GetSM_Quill)
        (:Is%20Valid
          (switch Utilities|FlowControl|Switch|SwitchonETimelineDirection _direction
            (:Forward
              (Utilities|FlowControl|Delay 1.0)
              (CallFunction|ReturnQuill))
            (:Backward
              (Class|BPIDamageable|DealDamage(Message) (Variables|Default|GetQuillTarget) (Variables|Default|GetQuillDamage))
              (Actor|DestroyActor))))
        (:Is%20Not%20Valid
          (Actor|DestroyActor))))))

(event EventBeginPlay
  (bind _quilltarget (Variables|Default|GetQuillTarget))
  (Utilities|IsValid _quilltarget
    (:Is%20Valid
      (Utilities|Array|RemoveItem (Variables|Default|GetAllQuillTargets) _quilltarget)
      (CallFunction|AimatTarget)
      (Actor|SetLifeSpan 6.0))
    (:Is%20Not%20Valid
      (Development|PrintString "BP_HedgehogQuill: Target not valid"))))

(fn ConstructionScript)