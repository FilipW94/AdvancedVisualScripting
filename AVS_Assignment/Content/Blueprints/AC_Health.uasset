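; Actor component that tracks an owner's health, starting CurrentHealth at MaxHealth on BeginPlay.
; HealthIncreased adds healing, clamped between zero and MaxHealth.
; HealthDecreased tests whether damage would bring health to zero or below and branches to OwnerDied or DamagedButAlive, without storing the reduced value.
; Both of those outcome functions are empty stubs.
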(event EventBeginPlay
  (Variables|Default|SetCurrentHealth (Variables|Default|GetMaxHealth)))

(fn HealthDecreased
  (params (DamageTaken :type Float%20%28double-precision%29))
  (if (<= (- (Variables|Default|GetCurrentHealth) DamageTaken) 0.0)
    (CallFunction|OwnerDied)
    (else
      (CallFunction|DamagedButAlive))))

(fn HealthIncreased
  (params (DamageHealed :type Float%20%28double-precision%29))
  (Variables|Default|SetCurrentHealth (Math|Float|Clamp(Float) (+ (Variables|Default|GetCurrentHealth) DamageHealed) 0.0 (Variables|Default|GetMaxHealth)))
  (return))

(fn OwnerDied
  (return))

(fn DamagedButAlive)