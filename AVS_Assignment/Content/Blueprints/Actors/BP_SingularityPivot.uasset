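; BP_SingularityPivot is an actor that pulls its attached enemy into the center of a singularity and damages it.
; On BeginPlay, a Drag timeline lerps the enemy horizontally toward the pivot, keeping its starting height.
; Once the enemy is within range, a FinalPull timeline takes over and lerps it into the pivot's location.
; During that pull, every update inside a smaller radius sends the enemy a damage message.
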(event Custom|DragTarget
  (bind _returnvalue (Transformation|GetActorLocation))
  (bind _attachedenemy (Variables|Default|GetAttachedEnemy))
  (bind _enemystartingposition (Variables|Default|GetEnemyStartingPosition))
  ;[0.15 0.15 0.15 0.5] Move enemy towards the bottom of the singularity
  (bind _pulltrack (Timeline|Drag PlayFromStart)
    (:Update
      (Utilities|IsValid _attachedenemy
        (:Is%20Valid
          (Transformation|SetActorLocation _attachedenemy (Math|Vector|Lerp(Vector) (Math|Vector|MakeVector (.x _enemystartingposition) (.y _enemystartingposition) (.z _enemystartingposition)) (Math|Vector|MakeVector (.x _returnvalue) (.y _returnvalue) (.z _enemystartingposition)) _pulltrack) false false)
          (if (CallFunction|IsEnemytoClose 7.5e+02)
            (CallFunction|StopDrag)
            (Variables|Default|SetFinalPullStartLocation (Transformation|GetActorLocation (Variables|Default|GetAttachedEnemy)))
            (CallFunction|FinalPull)))))))

(event Custom|FinalPull
  (bind _attachedenemy (Variables|Default|GetAttachedEnemy))
  ;[0.15 0.15 0.15 0.5] Move enemy into center
  (bind _pulltrack (Timeline|FinalPullTimeline PlayFromStart)
    (:Update
      (Utilities|IsValid _attachedenemy
        (:Is%20Valid
          (Transformation|SetActorLocation _attachedenemy (Math|Vector|Lerp(Vector) (Variables|Default|GetFinalPullStartLocation) (Transformation|GetActorLocation) _pulltrack) false false)
          (if (CallFunction|IsEnemytoClose 2.5e+02)
            (Class|BPIDamageable|DealDamage(Message) _attachedenemy 5e+01)))))))

(event Custom|StopDrag
  (bind _returnvalue (Transformation|GetActorLocation))
  (bind _attachedenemy (Variables|Default|GetAttachedEnemy))
  (bind _enemystartingposition (Variables|Default|GetEnemyStartingPosition))
  ;[0.15 0.15 0.15 0.5] Move enemy towards the bottom of the singularity
  (bind _pulltrack (Timeline|Drag Stop)
    (:Update
      (Utilities|IsValid _attachedenemy
        (:Is%20Valid
          (Transformation|SetActorLocation _attachedenemy (Math|Vector|Lerp(Vector) (Math|Vector|MakeVector (.x _enemystartingposition) (.y _enemystartingposition) (.z _enemystartingposition)) (Math|Vector|MakeVector (.x _returnvalue) (.y _returnvalue) (.z _enemystartingposition)) _pulltrack) false false)
          (if (CallFunction|IsEnemytoClose 7.5e+02)
            (CallFunction|StopDrag)
            (Variables|Default|SetFinalPullStartLocation (Transformation|GetActorLocation (Variables|Default|GetAttachedEnemy)))
            (CallFunction|FinalPull)))))))

(event Custom|StopFinalPull
  (bind _attachedenemy (Variables|Default|GetAttachedEnemy))
  ;[0.15 0.15 0.15 0.5] Move enemy into center
  (bind _pulltrack (Timeline|FinalPullTimeline Stop)
    (:Update
      (Utilities|IsValid _attachedenemy
        (:Is%20Valid
          (Transformation|SetActorLocation _attachedenemy (Math|Vector|Lerp(Vector) (Variables|Default|GetFinalPullStartLocation) (Transformation|GetActorLocation) _pulltrack) false false)
          (if (CallFunction|IsEnemytoClose 2.5e+02)
            (Class|BPIDamageable|DealDamage(Message) _attachedenemy 5e+01)))))))

(event EventBeginPlay
  (CallFunction|DragTarget))

(fn ConstructionScript)

(fn IsEnemytoClose
  (params (Range :type Float%20%28double-precision%29))
  (return (<= (Math|Vector|Distance(Vector) (Transformation|GetActorLocation (Variables|Default|GetAttachedEnemy)) (Transformation|GetActorLocation)) Range)))