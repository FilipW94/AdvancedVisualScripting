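; BP_StepSphere is an actor with a sphere mesh that grows and shrinks on command, then removes itself.
; Expand plays ScaleTimeline forward to lerp the mesh's relative scale from StartScale to FullScale, and Collapse reverses it from the end.
; The timeline's finish branches on direction: forward fires ExpandComplete after a short delay, while backward fires ShrinkComplete and destroys the actor.
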(event Custom|Collapse
  (bind (_direction _scaletrack) (Timeline|ScaleTimeline ReverseFromEnd)
    (:Update
      (Transformation|SetRelativeScale3D (Variables|Default|GetSM_Sphere) (Math|Vector|Lerp(Vector) (Variables|Default|GetStartScale) (Variables|Default|GetFullScale) _scaletrack)))
    (:Finished
      (switch Utilities|FlowControl|Switch|SwitchonETimelineDirection _direction
        (:Forward
          (Utilities|FlowControl|Delay 1.0)
          (Default|CallExpandComplete))
        (:Backward
          (Default|CallShrinkComplete)
          (Actor|DestroyActor))))))

(event Custom|Expand
  (bind (_direction _scaletrack) (Timeline|ScaleTimeline PlayFromStart)
    (:Update
      (Transformation|SetRelativeScale3D (Variables|Default|GetSM_Sphere) (Math|Vector|Lerp(Vector) (Variables|Default|GetStartScale) (Variables|Default|GetFullScale) _scaletrack)))
    (:Finished
      (switch Utilities|FlowControl|Switch|SwitchonETimelineDirection _direction
        (:Forward
          (Utilities|FlowControl|Delay 1.0)
          (Default|CallExpandComplete))
        (:Backward
          (Default|CallShrinkComplete)
          (Actor|DestroyActor))))))

(fn ConstructionScript)