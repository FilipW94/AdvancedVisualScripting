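; Spawner actor that creates a BP_TargetableActor enemy at the transform of each valid actor in EnemySpawnArray on BeginPlay.
; Spawned enemies are tracked in EnemyArray, and the EnemiesSpawned dispatcher fires after the spawn pass.
; RemoveAllEnemies destroys the tracked actors and fires EnemiesCleared, but does not empty the array.
; Both dispatchers fire only when their respective array is non-empty.
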(event EventBeginPlay
  (CallFunction|SpawnEnemiesatPoints))

(fn ConstructionScript)

(fn RemoveAllEnemies
  (bind _enemyarray (Variables|Default|GetEnemyArray))
  (if (Utilities|Array|IsNotEmpty _enemyarray)
    (for _array_element _enemyarray
      (Utilities|IsValid _array_element
        (:Is%20Valid
          (Actor|DestroyActor _array_element))))
    (Default|CallEnemiesCleared)))

(fn SpawnEnemiesatPoints
  (bind _enemyspawnarray (Variables|Default|GetEnemySpawnArray))
  (if (Utilities|Array|IsNotEmpty _enemyspawnarray)
    (for _array_element _enemyspawnarray
      (Utilities|IsValid _array_element
        (:Is%20Valid
          (bind _returnvalue (Game|SpawnActorfromClass "/Game/Blueprints/Actors/BP_TargetableActor.BP_TargetableActor_C" (Transformation|GetActorTransform _array_element) "AlwaysSpawn" "MultiplyWithRoot" 0 0))
          (Utilities|Array|AddUnique (Variables|Default|GetEnemyArray) _returnvalue))))
    (Default|CallEnemiesSpawned)))