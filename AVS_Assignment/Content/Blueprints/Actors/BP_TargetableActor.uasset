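; Targetable enemy actor with a health component and a random numeric ID label, used by the player's targeting system.
; A one-second timer checks player distance and adds or removes it from BP_TargetManager's target array.
; Damage events report health to the manager, while death removes it and clears main target and player focus if needed.
; The death animation drives a dynamic material's dissolve parameter through a timeline, then destroys the actor.
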(event Custom|EnemyDamagedButAlive_Event
  (bind _ac_health_enemy (Variables|Default|GetAC_Health_Enemy))
  (Default|TargetDamaged (Variables|Default|GetTargetManagerRef) (Variables|Default|GetTargetIdentifier) (Variables|/Game/Blueprints/ActorComponents/AC_Health_Base.AC_Health_Base_C|GetCurrentHealth _ac_health_enemy) (Variables|/Game/Blueprints/ActorComponents/AC_Health_Base.AC_Health_Base_C|GetMaxHealth _ac_health_enemy)))

(event Custom|DeathAnimation
  (Development|SetHiddeninGame (Variables|Default|GetTEXT_TargetIdentifier) true false)
  (Rendering|SetCastShadow (Variables|Default|GetSM_TargetableActor) false)
  (bind _returnvalue (Rendering|Material|CreateDynamicMaterialInstance (Variables|Default|GetSM_TargetableActor) 0 (Rendering|Material|GetMaterial (Variables|Default|GetSM_TargetableActor) 0) "None" :!class /Script/Engine.PrimitiveComponent))
  (bind _disintlerptrack (Timeline|DeathAnimationTimeline Play)
    (:Update
      (Rendering|Material|SetScalarParameterValue _returnvalue "Amount" (Math|Float|Lerp 0.0 1.0 _disintlerptrack) :!class /Script/Engine.MaterialInstanceDynamic))
    (:Finished
      (Actor|DestroyActor))))

(event Custom|PlayerDeathAnimation_Event
  (CallFunction|DeathAnimation))

(event Custom|NotifyPlayerDeath_Event
  (CallFunction|HandleTargetDeath))

(event EventBeginPlay
  (CallFunction|RandomizeIdentifier)
  (Rendering|Components|TextRender|SetText (Variables|Default|GetTEXT_TargetIdentifier) (Variables|Default|GetTargetIdentifier))
  (bind _returnvalue (Actor|GetActorOfClass "/Game/Blueprints/Actors/BP_TargetManager.BP_TargetManager_C"))
  (Variables|Default|SetTargetManagerRef _returnvalue)
  (CallFunction|CheckifinPlayerRange)
  (EventDispatchers|AssignNotifyOwnerDeath (Variables|Default|GetAC_Health_Enemy) (delegate Custom|NotifyPlayerDeath_Event))
  (EventDispatchers|AssignNotifyEnemyDamaged (Variables|Default|GetAC_Health_Enemy) (delegate Custom|EnemyDamagedButAlive_Event))
  (EventDispatchers|AssignPlayerDeathAnimation (Variables|Default|GetAC_Health_Enemy) (delegate Custom|PlayerDeathAnimation_Event)))

(event EventDealDamage
  (params (DamageDealt :type Float%20%28double-precision%29))
  (Default|HealthDecreased (Variables|Default|GetAC_Health_Enemy) DamageDealt))

(fn ConstructionScript)

(fn RandomizeIdentifier
  (Variables|Default|SetTargetIdentifier (Utilities|Text|ToText(String) (Utilities|String|ToString(Integer) (Math|Random|RandomIntegerinRange 0 999))))
  (return))

(fn CheckifinPlayerRange
  (if (>= (Math|Vector|Distance(Vector) (Transformation|GetActorLocation) (Transformation|GetActorLocation (Game|GetPlayerCharacter 0))) (Variables|Default|GetPlayerRange))
    (if (Variables|Default|GetDebugOn)
      (Rendering|Debug|DrawDebugSphere (Transformation|GetActorLocation) 1e+02 12 "(R=1.000000,G=0.030547,B=0.000000,A=1.000000)" 5.0))
    (CallFunction|NotinPlayerRange)
    (else
      (if (Variables|Default|GetDebugOn)
        (Rendering|Debug|DrawDebugSphere (Transformation|GetActorLocation) 1e+02 12 "(R=0.140633,G=1.000000,B=0.000000,A=1.000000)" 5.0))
      (CallFunction|InPlayerRange))))

(fn NotinPlayerRange
  (if (Utilities|Array|ContainsItem (Variables|/Game/Blueprints/Actors/BP_TargetManager.BP_TargetManager_C|GetTargetableActors (Variables|Default|GetTargetManagerRef)) self)
    (Default|RemoveTargetfromArray (Variables|Default|GetTargetManagerRef) self))
  (Utilities|Time|SetTimerbyFunctionName 0 "CheckIfInPlayerRange" 1.0))

(fn InPlayerRange
  (if (Utilities|Array|ContainsItem (Variables|/Game/Blueprints/Actors/BP_TargetManager.BP_TargetManager_C|GetTargetableActors (Variables|Default|GetTargetManagerRef)) self)
    _
    (else
      (Default|AddTargettoArray (Variables|Default|GetTargetManagerRef) self)))
  (Utilities|Time|SetTimerbyFunctionName 0 "CheckIfInPlayerRange" 1.0))

(fn HandleTargetDeath
  (Default|RemoveTargetfromArray (Variables|Default|GetTargetManagerRef) self)
  (if (== (Variables|/Game/Blueprints/Actors/BP_TargetManager.BP_TargetManager_C|GetCurrentMainTarget (Variables|Default|GetTargetManagerRef)) self)
    (Default|ClearMainTarget (Variables|Default|GetTargetManagerRef))
    (Utilities|StopPlayerfromFocusing)
    (Default|CleanupDoneEvent (Variables|Default|GetAC_Health_Enemy))
    (return)
    (else
      (Default|CleanupDoneEvent (Variables|Default|GetAC_Health_Enemy)))))

(fn GetHealth
  (return (Variables|/Game/Blueprints/ActorComponents/AC_Health_Base.AC_Health_Base_C|GetCurrentHealth (Variables|Default|GetAC_Health_Enemy))))

(fn GetTarget
  (bind _ac_health_enemy (Variables|Default|GetAC_Health_Enemy))
  (return (Variables|Default|GetTargetIdentifier) (Variables|/Game/Blueprints/ActorComponents/AC_Health_Base.AC_Health_Base_C|GetCurrentHealth _ac_health_enemy) (Variables|/Game/Blueprints/ActorComponents/AC_Health_Base.AC_Health_Base_C|GetMaxHealth _ac_health_enemy)))