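; Base projectile actor that homes in on a target actor and deals damage to what it hits.
; On BeginPlay a timeline lerps the projectile mesh from its spawn location to the target's current position, destroying the actor if the target becomes invalid.
; Overlapping an actor that implements BPI_Damageable sends it a damage message and destroys the projectile, which otherwise has a limited lifespan.
; Spline path and debug-draw logic is present but never called.
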(event Custom|Create%20Spline
  (bind _targetactor (Variables|Default|GetTargetActor))
  (bind _sm_projectile (Variables|Default|GetSM_Projectile))
  (bind _returnvalue (Transformation|GetWorldLocation _sm_projectile))
  (bind _returnvalue_2 (Transformation|GetActorLocation _targetactor))
  (if (Variables|Default|GetMoveProjectile)
    (bind _returnvalue_3 (AddComponent|AddSplineComponent false (Math|Transform|MakeTransform (Variables|Default|GetSpawnLocation) "0, 0, 0" "1.000000,1.000000,1.000000")))
    (bind _output_get (Variables|Default|SetSplineComponent _returnvalue_3))
    (Spline|AddSplinePoint _output_get _returnvalue "World" true)
    (Spline|AddSplinePoint _output_get _returnvalue_2 "World" true)
    (Class|SplineComponent|SetDrawDebug _output_get true)
    (Rendering|Debug|DrawDebugSphere _returnvalue 1e+02 12 "(R=1.000000,G=1.000000,B=1.000000,A=1.000000)" 1e+01)
    (Rendering|Debug|DrawDebugSphere _returnvalue_2 1e+02 12 "(R=1.000000,G=1.000000,B=1.000000,A=1.000000)" 11.0)))

(event Custom|MoveAlongSpline)

(event Custom|MoveToTarget
  (bind _targetactor (Variables|Default|GetTargetActor))
  (bind _lerptrack (Timeline|Timeline Play)
    (:Update
      (Utilities|IsValid _targetactor
        (:Is%20Valid
          (Transformation|SetWorldLocation (Variables|Default|GetSM_Projectile) (Math|Vector|Lerp(Vector) (Variables|Default|GetSpawnLocation) (Transformation|GetActorLocation _targetactor) _lerptrack) false false))
        (:Is%20Not%20Valid
          (Actor|DestroyActor))))))

(event EventBeginPlay
  (Actor|SetLifeSpan 1e+01)
  (Variables|Default|SetSpawnLocation (Transformation|GetActorLocation))
  (Variables|Default|SetMoveProjectile true)
  (CallFunction|MovetoTarget))

(event Collision|EventActorBeginOverlap
  (params (OtherActor :type Actor%20Object%20Reference))
  (if (Utilities|DoesObjectImplementInterface OtherActor "/Game/Blueprints/Interfaces/BPI_Damageable.BPI_Damageable_C")
    (Class|BPIDamageable|DealDamage(Message) OtherActor (Variables|Default|GetDamageDealth))
    (Actor|DestroyActor)))

(event EventTick
  (params (DeltaSeconds :type Float%20%28single-precision%29)))

(fn ConstructionScript)