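; Target manager actor that tracks targetable actors and the current main target, mirroring both in a lazily created WBP_TargetManagerUI.
; Registration accepts BPI_Targetable actors, whose target messages supply the identifier and health shown in the widget.
; Distance searches return the closest actor in a radius, promoting it to main target, or up to N nearest within range.
; A static mesh marker moves above the main target and hides when cleared.
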(event EventBeginPlay
  (Development|SetHiddeninGame (Variables|Default|GetSM_TargetMarker) true false))

(fn ConstructionScript)

(fn AddTargettoArray
  (params (NewTarget :type Actor%20Object%20Reference))
  (if (Utilities|DoesObjectImplementInterface NewTarget "/Game/Blueprints/Interfaces/BPI_Targetable.BPI_Targetable_C")
    (Utilities|Array|Add (Variables|Default|GetTargetableActors) NewTarget)
    (bind (_targetidentifier _currenthealth _maxhealth) (Class|BPITargetable|GetTarget(Message) NewTarget))
    (CallFunction|ValidateWidget)
    (Default|AddTargettoList (Variables|Default|GetTargetManagerUIREF) (Utilities|Text|ToText(String) (Utilities|GetDisplayName NewTarget)) _targetidentifier _currenthealth _maxhealth)
    (return)))

(fn ValidateWidget
  (Utilities|IsValid (Variables|Default|GetTargetManagerUIREF)
    (:Is%20Valid
      (return))
    (:Is%20Not%20Valid
      (bind _returnvalue (UserInterface|CreateWidget "/Game/Widgets/WBP_TargetManagerUI.WBP_TargetManagerUI_C" (Game|GetPlayerController 0)))
      (bind _output_get (Variables|Default|SetTargetManagerUIREF _returnvalue))
      (UserInterface|Viewport|AddtoViewport _output_get 0)
      (return))))

(fn RemoveTargetfromArray
  (params (TargetToRemove :type Actor%20Object%20Reference))
  (bind _targetidentifier (Class|BPITargetable|GetTarget(Message) TargetToRemove))
  (CallFunction|ValidateWidget)
  (Default|RemoveTargetfromList (Variables|Default|GetTargetManagerUIREF) _targetidentifier)
  (bind _returnvalue (Utilities|Array|RemoveItem (Variables|Default|GetTargetableActors) TargetToRemove))
  (Development|PrintString (Utilities|String|ToString(Boolean) _returnvalue))
  (return))

(fn FindClosestTargettoLocation
  (params (SourcePoint :type Vector) (SearchRadius :type Float%20%28double-precision%29))
  (for _array_element (Variables|Default|GetTargetableActors)
    (Utilities|IsValid _array_element
      (:Is%20Valid
        (if (<= (Math|Vector|Distance(Vector) SourcePoint (Transformation|GetActorLocation _array_element)) SearchRadius)
          (if (<= (Math|Vector|Distance(Vector) SourcePoint (Transformation|GetActorLocation _array_element)) (LocalVariables|GetCurrentMinDistance))
            (LocalVariables|SetCurrentMinDistance (Math|Vector|Distance(Vector) SourcePoint (Transformation|GetActorLocation _array_element)))
            (LocalVariables|SetClosestActor _array_element))))))
  (Utilities|IsValid (LocalVariables|GetClosestActor)
    (:Is%20Valid
      (CallFunction|SetNewMainTarget (LocalVariables|GetClosestActor))
      (return (LocalVariables|GetClosestActor)))
    (:Is%20Not%20Valid
      (return 0))))

(fn SetNewMainTarget
  (params (NewMainTarget :type Actor%20Object%20Reference))
  (bind _returnvalue (Transformation|GetActorLocation NewMainTarget))
  (bind _output_get (Variables|Default|SetCurrentMainTarget NewMainTarget))
  (bind (_targetidentifier _currenthealth _maxhealth) (Class|BPITargetable|GetTarget(Message) _output_get))
  (Default|SetMainTarget (Variables|Default|GetTargetManagerUIREF) (Utilities|Text|ToText(String) (Utilities|GetDisplayName NewMainTarget)) _targetidentifier _currenthealth _maxhealth)
  (Transformation|SetWorldLocation (Variables|Default|GetSM_TargetMarker) (Math|Vector|MakeVector (.x _returnvalue) (.y _returnvalue) (+ (.z _returnvalue) (Variables|Default|GetMarkerHeightOffset))) false true)
  (Development|SetHiddeninGame (Variables|Default|GetSM_TargetMarker) false false))

(fn ClearMainTarget
  (Default|ClearOldMainTarget (Variables|Default|GetTargetManagerUIREF))
  (Development|SetHiddeninGame (Variables|Default|GetSM_TargetMarker) true false)
  (return))

(fn TargetDamaged
  (params (TargetIdentifier :type Text) (CurrentHealth :type Float%20%28double-precision%29) (MaxHealth :type Float%20%28double-precision%29))
  (Default|SetTargetinArrayHealth (Variables|Default|GetTargetManagerUIREF) TargetIdentifier CurrentHealth MaxHealth)
  (return))

(fn FindClosestTargets
  (params (SourceLocation :type Vector) (MaxRange :type Float%20%28double-precision%29) (AmountOfTargets :type Integer))
  (bind _closesttargets (LocalVariables|GetClosestTargets))
  (bind _targetableactors (Variables|Default|GetTargetableActors))
  (bind _returnvalue (Utilities|Array|Length _targetableactors))
  (bind _output_get (LocalVariables|SetTargetableArrayCopy (Variables|Default|GetTargetableActors)))
  (if (<= _returnvalue AmountOfTargets)
    (LocalVariables|SetTargetsInArray _returnvalue)
    (else
      (LocalVariables|SetTargetsInArray AmountOfTargets)))
  (Utilities|FlowControl|ForLoopwithBreak 0 (- (LocalVariables|GetTargetsInArray) 1)
    (:LoopBody
      (for _array_element _output_get
        (Utilities|IsValid _array_element
          (:Is%20Valid
            (if (<= (Math|Vector|Distance(Vector) (Transformation|GetActorLocation _array_element) SourceLocation) (LocalVariables|GetCurrentClosestDistance))
              (if (<= (Math|Vector|Distance(Vector) (Transformation|GetActorLocation _array_element) SourceLocation) MaxRange)
                (LocalVariables|SetCurrentClosestDistance (Math|Vector|Distance(Vector) (Transformation|GetActorLocation _array_element) SourceLocation))
                (LocalVariables|SetClosestActor _array_element))))))
      (Utilities|Array|AddUnique (LocalVariables|GetClosestTargets) (LocalVariables|GetClosestActor))
      (Utilities|Array|RemoveItem (LocalVariables|GetTargetableArrayCopy) (LocalVariables|GetClosestActor))
      (LocalVariables|SetCurrentClosestDistance 1e+04))
    (:Completed
      (if (Utilities|Array|IsNotEmpty _closesttargets)
        (return _closesttargets)
        (else
          (Development|PrintString "No targets in range"))))))