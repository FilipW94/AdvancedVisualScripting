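; BP_MaterialTestCube is a test actor that animates a material parameter on its static mesh and then destroys itself.
; Two seconds after BeginPlay it turns off shadow casting and creates a dynamic material instance from the mesh's first material.
; A timeline drives that instance's Amount scalar between zero and one, and the actor is destroyed when the timeline finishes.
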(event EventBeginPlay
  (Utilities|FlowControl|Delay 2.0)
  (Rendering|SetCastShadow (Variables|Default|GetStaticMesh) false)
  (bind _returnvalue (Rendering|Material|CreateDynamicMaterialInstance (Variables|Default|GetStaticMesh) 0 (Rendering|Material|GetMaterial (Variables|Default|GetStaticMesh) 0) "None" :!class /Script/Engine.PrimitiveComponent))
  (bind _newtrack_0 (Timeline|Timeline Play)
    (:Update
      (Rendering|Material|SetScalarParameterValue _returnvalue "Amount" (Math|Float|Lerp 0.0 1.0 _newtrack_0) :!class /Script/Engine.MaterialInstanceDynamic))
    (:Finished
      (Actor|DestroyActor))))

(fn ConstructionScript)