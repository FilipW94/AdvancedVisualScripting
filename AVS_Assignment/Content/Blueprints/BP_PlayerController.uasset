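; Player controller that creates the game menu widget and manages its visibility.
; On BeginPlay it stores a WBP_GameMenu instance, pauses the game and shows the menu with cursor usage enabled.
; The IA_PauseMenu input toggles the menu on and off the viewport along with cursor usage, without changing the pause state.
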(event Input|EnhancedActionEvents|EnhancedInputActionIA_PauseMenu
  (params (ActionValue :type Boolean) (ElapsedSeconds :type Float%20%28double-precision%29) (TriggeredSeconds :type Float%20%28double-precision%29) (InputAction :type Input%20Action%20Object%20Reference :default "/Game/Inputs/IA_PauseMenu.IA_PauseMenu"))
  (bind _pausemenuref (Variables|Default|GetPauseMenuRef))
  (:Triggered
    (if (UserInterface|Viewport|IsinViewport (Variables|Default|GetPauseMenuRef))
      (Widget|RemovefromParent _pausemenuref)
      (CallFunction|SetCursorUsage false)
      (else
        (UserInterface|Viewport|AddtoViewport _pausemenuref 0)
        (CallFunction|SetCursorUsage true)))))

(event EventBeginPlay
  (bind _returnvalue (UserInterface|CreateWidget "/Game/Widgets/WBP_GameMenu.WBP_GameMenu_C" (Game|GetPlayerController 0)))
  (bind _output_get (Variables|Default|SetPauseMenuRef _returnvalue))
  (Game|SetGamePaused true)
  (UserInterface|Viewport|AddtoViewport _output_get 0)
  (CallFunction|SetCursorUsage true))

(fn ConstructionScript)